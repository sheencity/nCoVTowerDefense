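; Bat enemy that flies along a level spline, then fires virus projectiles on a looping timer.
; A timeline drives it to a randomized offset and end distance; on finishing it picks one of two random yaw ranges and repeatedly spawns BP_Virus at the muzzle.
; Damage updates a widget health bar; death awards coins through BP_CoinManager, notifies the player controller and destroys the bat.
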(event Custom|Enable%20Fire
  (bind _capsulecomponent (Variables|Default|GetCapsuleComponent))
  (if (>= (Math|Random|RandomIntegerinRange 0 5) 3)
    ;[1 1 1] 开始射击
    (Transformation|SetWorldRotation _capsulecomponent (Math|Rotator|MakeRotator 0.0 0.0 (Math|Conversions|ToFloat(Integer) (Math|Random|RandomIntegerinRange -100 -90))) false false)
    (else
      (Transformation|SetWorldRotation _capsulecomponent (Math|Rotator|MakeRotator 0.0 0.0 (Math|Conversions|ToFloat(Integer) (Math|Random|RandomIntegerinRange -72 -62))) false false)))
  (if (not (Variables|Default|GetisAttacking))
    (Variables|Default|SetisAttacking true)
    (bind _returnvalue (Utilities|Time|SetTimerbyEvent (EventDispatchers|CreateEvent :!event Custom|Fire) (/ 6e+01 (Math|Conversions|ToFloat(Integer) (Variables|Default|GetRate))) true))
    (Variables|Default|SetFire%20Timer _returnvalue)))

(event Custom|Disable%20Fire
  ;[1 1 1] 停止开火
  (if (Variables|Default|GetisAttacking)
    (Utilities|Time|ClearandInvalidateTimerbyHandle (Variables|Default|GetFire%20Timer))
    (Variables|Default|SetisAttacking false)))

(event Custom|Fire
  (CallFunction|Attack))

(event EventBeginPlay
  ;[1 1 1] 获取曲线
  (bind _outactors (Actor|GetAllActorsOfClass "/Game/Blueprints/Spline.Spline_C"))
  (Variables|Default|SetSpline (Utilities|Array|Get(acopy) _outactors))
  (bind _asblood_3d (Utilities|Casting|CastToBlood3D (UserInterface|GetUserWidgetObject (Variables|Default|GetWidget))))
  (bind _output_get (Variables|Default|SetBlood _asblood_3d))
  (bind _output_get_2 (Variables|Default|SetCurrentHealth (Variables|Default|GetMaxHealth)))
  (Progress|SetPercent (Variables|/Game/Blueprints/Blood3D.Blood3D_C|GetProgressBar_26 _output_get) _output_get_2)
  (bind _outactors_2 (Actor|GetAllActorsOfClass "/Game/Blueprints/BP_CoinManager.BP_CoinManager_C"))
  (Variables|Default|SetCoinManager (Utilities|Array|Get(acopy) _outactors_2))
  ;[1 1 1] 随机偏移值
  (Variables|Default|SetRandomOffset (Math|Random|RandomIntegerinRange -50 50))
  ;[1 1 1] 随机终点位置distance
  (Variables|Default|SetRandomDistance (Math|Random|RandomFloatinRange 0.96 1.0))
  ;[1 1 1] 50秒
  (bind _newtrack_0 (Timeline|Timeline_0 PlayFromStart)
    (:Update
      (Transformation|SetActorLocationAndRotation (.ReturnValue (Default|GetLocationandRotation (Variables|Default|GetSpline) (Math|Float|Lerp 0.0 (Variables|Default|GetRandomDistance) _newtrack_0) (Variables|Default|GetRandomOffset))) (.ReturnValue1 (Default|GetLocationandRotation (Variables|Default|GetSpline) (Math|Float|Lerp 0.0 (Variables|Default|GetRandomDistance) _newtrack_0) (Variables|Default|GetRandomOffset)))))
    (:Finished
      (CallFunction|EnableFire))))

(event Game|Damage|EventAnyDamage
  (params (Damage :type Float%20%28single-precision%29) (DamageType :type Damage%20Type%20Object%20Reference) (InstigatedBy :type Controller%20Object%20Reference) (DamageCauser :type Actor%20Object%20Reference))
  ;[1 1 1] Receive Damage
  (bind _output_get (Variables|Default|SetCurrentHealth (Math|Conversions|ToFloat(Integer) (- (Math|Float|Truncate (stale _output_get)) (Math|Float|Truncate Damage))))) ; reduce health
  (Progress|SetPercent (Variables|/Game/Blueprints/Blood3D.Blood3D_C|GetProgressBar_26 (Variables|Default|GetBlood)) (/ (Variables|Default|GetCurrentHealth) (Variables|Default|GetMaxHealth)))
  (if (<= (Math|Float|Truncate _output_get) 0) ; if health is 0 or less
    (Default|AddCoin (Variables|Default|GetCoinManager) (Variables|Default|GetPrice))
    (Default|OnEnemyDead (.AsN%20Cov%20Controller (Utilities|Casting|CastTonCov_Controller (Game|GetPlayerController 0))))
    (Actor|DestroyActor) ; destroy unit
  ))

(fn ConstructionScript)

(fn Attack
  (Game|SpawnActorfromClass "/Game/Blueprints/BP_Virus.BP_Virus_C" (Transformation|GetWorldTransform (Variables|Default|GetMuzzle)) "Undefined" 0 5e+02 1e+02 0)
  (Audio|PlaySound2D "/Game/Audio/hit.hit" 1.0 1.0 0.0 0 0))