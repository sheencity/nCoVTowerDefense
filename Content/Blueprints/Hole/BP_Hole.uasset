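; BP_Hole is a tower build slot that the player buys for 100 coins, replacing itself with a BP_BaseTower.
; Its Paper sprite starts hidden, shows with a tint and sound on hover, and opens a BP_BuyTower widget component when clicked.
; The widget's click event asks BP_CoinManager to consume coins, then spawns the tower and destroys the hole; its mouse-leave event hides the widget.
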(event OnBeginCursorOver(PaperSprite)
  (params (TouchedComponent :type Primitive%20Component%20Object%20Reference))
  (Sprite|SetSpriteColor (Variables|Default|GetPaperSprite) "(R=0.875000,G=0.755947,B=0.050130,A=1.000000)")
  (CallFunction|SetHoleVisibility true)
  (Audio|PlaySound2D "/Game/Audio/Click.Click" 3.0 1.0 0.0 0 0))

(event OnEndCursorOver(PaperSprite)
  (params (TouchedComponent :type Primitive%20Component%20Object%20Reference))
  (Sprite|SetSpriteColor (Variables|Default|GetPaperSprite) "(R=1.000000,G=1.000000,B=1.000000,A=1.000000)")
  (CallFunction|SetHoleVisibility false))

(event OnClicked(PaperSprite)
  (params (TouchedComponent :type Primitive%20Component%20Object%20Reference) (ButtonPressed :type Key%20Structure :default "None"))
  (Sprite|SetSpriteColor (Variables|Default|GetPaperSprite) "(R=0.190726,G=0.875000,B=0.116132,A=1.000000)")
  (CallFunction|ShowBuyTower true)
  (Audio|PlaySound2D "/Game/Audio/Click.Click" 3.0 1.0 0.0 0 0))

(event Custom|MouseLeave_Disp_Event_0
  (CallFunction|ShowBuyTower false))

(event Custom|CustomEvent_0
  (bind _newparam (Default|ConsumeCoin (Variables|Default|GetCoinManager) 100))
  (if _newparam
    (Game|SpawnActorfromClass "/Game/Blueprints/Towers/BP_BaseTower.BP_BaseTower_C" (Math|Transform|MakeTransform (+ (Transformation|GetActorLocation) "0, 0,-20.000000") "0, 0, 0" "1,1,1") "AlwaysSpawn" 0 0)
    (Audio|PlaySound2D "/Game/Audio/Click2.Click2" 3.0 1.0 0.2 0 0)
    (Utilities|FlowControl|Delay 0.05)
    (Actor|DestroyActor self)))

(event EventBeginPlay
  (CallFunction|SetHoleVisibility false)
  (bind _asbp_buy_tower (Utilities|Casting|CastToBP_BuyTower (UserInterface|GetUserWidgetObject (Variables|Default|GetWidget))))
  (bind _outactors (Actor|GetAllActorsOfClass "/Game/Blueprints/BP_CoinManager.BP_CoinManager_C"))
  (Variables|Default|SetCoinManager (Utilities|Array|Get(acopy) _outactors))
  (EventDispatchers|BindEventtoClick _asbp_buy_tower (delegate Custom|CustomEvent_0))
  (EventDispatchers|AssignMouseLeaveDisp _asbp_buy_tower (delegate Custom|MouseLeave_Disp_Event_0)))

(fn ConstructionScript)

(fn ShowBuyTower
  (params (bNewVisibility :type Boolean))
  (Rendering|SetVisibility (Variables|Default|GetWidget) bNewVisibility false))

(fn SetHoleVisibility
  (params (Visibility :type Boolean))
  (Rendering|SetVisibility (Variables|Default|GetPaperSprite) Visibility false)
  (return))

(fn NewFunction1
  (params (Visibility :type Boolean))
  (bind _outactors (Actor|GetAllActorsOfClass "BP_Hole_C"))
  (for _array_element _outactors
    (CallFunction|SetHoleVisibility _array_element Visibility)))