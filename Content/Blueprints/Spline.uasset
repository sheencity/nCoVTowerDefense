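; Spline actor Blueprint that serves as a path, exposing a function to sample position and orientation along it.
; GetLocationAndRotation scales a normalized Distance by spline length, returning a world location shifted sideways by B and a rotation facing along the spline direction.
; The sideways offset uses the local-space right vector, while location and direction are world-space; the NewParam output is always false.
; Event graph and construction script contain no active logic.
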(event EventBeginPlay)

(event Collision|EventActorBeginOverlap
  (params (OtherActor :type Actor%20Object%20Reference)))

(event EventTick
  (params (DeltaSeconds :type Float%20%28single-precision%29)))

(fn ConstructionScript)

(fn GetLocationandRotation
  (params (Distance :type Float%20%28single-precision%29) (B :type Integer))
  (bind _spline (Variables|Default|GetSpline))
  (bind _returnvalue (Spline|GetSplineLength _spline))
  (bind _returnvalue_2 (* Distance _returnvalue))
  (return false (+ (Spline|GetLocationatDistanceAlongSpline _spline _returnvalue_2 "World") (* (Class|SplineComponent|GetRightVectoratDistanceAlongSpline _spline _returnvalue_2 "Local") B)) (Math|Conversions|RotationFromXVector (Spline|GetDirectionatDistanceAlongSpline _spline _returnvalue_2 "World"))))