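; Spawner actor that releases waves of Bat_AI enemies, sized per wave by the Nums array.
; Three seconds after BeginPlay, a looping one-second timer spawns one bat per tick until the current wave's count is reached, then clears itself.
; A second 30-second timer advances WaveIndex and restarts spawning until the array is exhausted.
; A random delay is stored on each spawn but never read here.
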(event Custom|CustomEvent_0
  (bind _index (Variables|Default|GetIndex))
  ;[1 1 1] 生成根据配置数量的野怪
  (if (< _index (Utilities|Array|Get(acopy) (Variables|Default|GetNums) (Variables|Default|GetWaveIndex)))
    (Game|SpawnActorfromClass "/Game/Blueprints/Bat_AI.Bat_AI_C" (Math|Transform|MakeTransform "0, 0, 0" "0, 0, 0" "1,1,1") "AlwaysSpawn" 0 0)
    (Math|Integer|IncrementInt _index
      (:%20%20
        (Variables|Default|SetRandomTIme (Math|Random|RandomFloatinRange 5.0 1e+01))))
    (else
      (Utilities|Time|ClearandInvalidateTimerbyHandle (Variables|Default|GetNewVar_0)))))

(event Custom|CustomEvent_1
  (bind _waveindex (Variables|Default|GetWaveIndex))
  (if (< _waveindex (Utilities|Array|Length (Variables|Default|GetNums)))
    (Math|Integer|IncrementInt _waveindex
      (:%20%20
        (Variables|Default|SetIndex 0)
        (bind _returnvalue (Utilities|Time|SetTimerbyEvent (delegate Custom|CustomEvent_0) 1.0 true))
        (Variables|Default|SetNewVar_0 _returnvalue)))
    (else
      (Utilities|Time|ClearandInvalidateTimerbyHandle (Variables|Default|GetNewVar_1)))))

(event EventBeginPlay
  (Utilities|FlowControl|Delay 3.0)
  (Utilities|FlowControl|Sequence
    (:then_0
      (Variables|Default|SetIndex 0)
      (bind _returnvalue (Utilities|Time|SetTimerbyEvent (delegate Custom|CustomEvent_0) 1.0 true))
      (Variables|Default|SetNewVar_0 _returnvalue))
    (:then_1
      ;[1 1 1] 每隔30秒生成一波野怪
      (bind _returnvalue_2 (Utilities|Time|SetTimerbyEvent (delegate Custom|CustomEvent_1) 3e+01 true))
      (Variables|Default|SetNewVar_1 _returnvalue_2))))

(fn ConstructionScript)