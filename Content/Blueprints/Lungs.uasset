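; Lungs actor that takes damage and triggers the game-over screen when its Health runs out.
; The construction script creates a dynamic material on the FeiMo mesh, and each hit remaps remaining Health into its BloodPercent parameter.
; At zero Health it sets the WBPOver state to false and shows that widget, reached through the MainUmg instance found on BeginPlay.
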(event EventBeginPlay
  (bind _foundwidgets (Widget|GetAllWidgetsOfClass "/Game/Blueprints/MainUmg.MainUmg_C" true))
  (Variables|Default|SetMainUMG (Utilities|Array|Get(acopy) _foundwidgets)))

(event Collision|EventActorBeginOverlap
  (params (OtherActor :type Actor%20Object%20Reference)))

(event EventTick
  (params (DeltaSeconds :type Float%20%28single-precision%29)))

(event Game|Damage|EventAnyDamage
  (params (Damage :type Float%20%28single-precision%29) (DamageType :type Damage%20Type%20Object%20Reference) (InstigatedBy :type Controller%20Object%20Reference) (DamageCauser :type Actor%20Object%20Reference))
  (bind _mainumg (Variables|Default|GetMainUMG))
  (bind _wbp_over (Variables|/Game/Blueprints/MainUmg.MainUmg_C|GetWBP_Over _mainumg))
  (bind _output_get (Variables|Default|SetHealth (- (Variables|Default|GetHealth) Damage)))
  (CallFunction|SetLungsBlood (Math|Float|MapRangeClamped _output_get 0.0 1e+04 0.0 1.0))
  (if (<= (Variables|Default|GetHealth) 0.0)
    (Default|SetState _wbp_over false)
    (Widget|SetVisibility _wbp_over "SelfHitTestInvisible")))

(fn ConstructionScript
  (bind _returnvalue (Rendering|Material|CreateDynamicMaterialInstance (Variables|Default|GetFei_mo) 0 0 "None" :!class /Script/Engine.PrimitiveComponent))
  (Variables|Default|SetMaterial _returnvalue))

(fn SetLungsBlood
  (params (Percent :type Float%20%28single-precision%29))
  (Rendering|Material|SetScalarParameterValue (Variables|Default|GetMaterial) "BloodPercent" Percent :!class /Script/Engine.MaterialInstanceDynamic))