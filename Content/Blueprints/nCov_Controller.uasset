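; nCov_Controller is a controller that runs the game flow from intro screen to the all-enemies-dead end state.
; On BeginPlay it shows FirstUMG in UI-only input and plays BGM.
; When FirstUMG's Finished dispatcher fires, it switches to game-and-UI input, creates MainUmg, spawns SpawnAI and stores its enemy total.
; OnEnemyDead decrements that count and sets MainUMG's over state to true at zero.
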(event Custom|Finished_Event_0
  (Input|SetInputModeGameandUI (Game|GetPlayerController 0) 0 "DoNotLock" true)
  (bind _returnvalue (UserInterface|CreateWidget "/Game/Blueprints/MainUmg.MainUmg_C"))
  (UserInterface|Viewport|AddtoViewport _returnvalue 0)
  (Variables|Default|SetMainUMG _returnvalue)
  (bind _returnvalue_2 (Game|SpawnActorfromClass "/Game/Blueprints/SpawnAI.SpawnAI_C" (Math|Transform|MakeTransform "0, 0, 0" "0, 0, 0" "1,1,1") "AlwaysSpawn" 0 0))
  (Variables|Default|SetSpawnAI _returnvalue_2)
  (Variables|Default|SetTotalEnemys (Default|GetTotalEnemy (Variables|Default|GetSpawnAI))))

(event EventBeginPlay
  (Input|SetInputModeUIOnly (Game|GetPlayerController 0) 0 "DoNotLock")
  (bind _returnvalue (UserInterface|CreateWidget "/Game/Blueprints/FirstUMG.FirstUMG_C"))
  (UserInterface|Viewport|AddtoViewport _returnvalue 0)
  (EventDispatchers|AssignFinished _returnvalue (delegate Custom|Finished_Event_0))
  (Audio|PlaySound2D "/Game/Audio/BGM.BGM" 1.0 1.0 0.0 0 0))

(fn ConstructionScript)

(fn OnEnemyDead
  (bind _totalenemys (Variables|Default|GetTotalEnemys))
  (Math|Integer|DecrementInt _totalenemys
    (:%20%20
      (if (<= _totalenemys 0)
        (Default|SetOverState (Variables|Default|GetMainUMG) true)))))