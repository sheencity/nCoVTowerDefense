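; BP_CoinManager holds the player's coin balance and keeps the main HUD display in sync with it.
; On BeginPlay it retries on a short delay until the nCov_Controller's MainUMG widget exists, then pushes the starting balance.
; AddCoin plays a sound and raises the balance, while ConsumeCoin deducts only when funds suffice and returns whether it succeeded.
; Both update the display through UpdateUMGCoin.
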(event EventBeginPlay
  (Variables|/Game/Blueprints/nCov_Controller.nCov_Controller_C|GetMainUMG (.AsN%20Cov%20Controller (Utilities|Casting|CastTonCov_Controller (Game|GetPlayerController 0))) :!label _label
    (:then
      (CallFunction|UpdateUMGCoin))
    (:else
      (Utilities|FlowControl|Delay 0.2)
      (goto _label))))

(fn ConstructionScript)

(fn AddCoin
  (params (Value :type Integer))
  (Audio|PlaySound2D "/Game/Audio/Coin2.Coin2" 1.0 1.0 0.0 0 0)
  (Variables|Default|SetCurrentCoin (+ (Variables|Default|GetCurrentCoin) Value))
  (CallFunction|UpdateUMGCoin))

(fn ConsumeCoin
  (params (Value :type Integer))
  (if (>= (- (Variables|Default|GetCurrentCoin) Value) 0)
    (Variables|Default|SetCurrentCoin (Math|Integer|Clamp(Integer) (- (Variables|Default|GetCurrentCoin) Value) 0 10000000))
    (CallFunction|UpdateUMGCoin)
    (return true)
    (else
      (return false))))

(fn UpdateUMGCoin
  (bind _mainumg (Variables|/Game/Blueprints/nCov_Controller.nCov_Controller_C|GetMainUMG (.AsN%20Cov%20Controller (Utilities|Casting|CastTonCov_Controller (Game|GetPlayerController 0))))
    (:then
      (Default|SetCoin _mainumg (Variables|Default|GetCurrentCoin)))
    (:else)))