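; Enemy manager Blueprint that tracks enemy deaths and shows the game-over widget when none remain.
; OnEnemyDead decrements its TotalEnemy, then reads the remaining count from the SpawnAI reference on the player's nCov_Controller.
; At zero or below, it sets the state of the main UMG's WBPOver widget to true, makes it visible and prints a debug string.
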(fn ConstructionScript)

(fn OnEnemyDead
  (bind _returnvalue (Game|GetPlayerController 0))
  (bind _asn_cov_controller (Utilities|Casting|CastTonCov_Controller _returnvalue))
  (bind _mainumg (Variables|/Game/Blueprints/nCov_Controller.nCov_Controller_C|GetMainUMG _asn_cov_controller))
  (bind _wbp_over (Variables|/Game/Blueprints/MainUmg.MainUmg_C|GetWBP_Over _mainumg))
  (Variables|Default|SetTotalEnemy (- (Variables|Default|GetTotalEnemy) 1))
  (if (<= (Default|GetTotalEnemy (Variables|/Game/Blueprints/nCov_Controller.nCov_Controller_C|GetSpawnAI _asn_cov_controller)) 0)
    (Default|SetState _wbp_over true)
    (Widget|SetVisibility _wbp_over "SelfHitTestInvisible")
    (Development|PrintString "Hello")))